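; Enemy character that patrols between random tagged actors and uses AI Perception to chase and melee the third-person player.
; A perception update raises walk speed and starts the chase; forgetting the player slows it and resumes patrol.
; On reaching the player it plays a charged-attack montage, whose notify sphere-traces forward to deal damage.
; Its Health component updates a widget health bar and destroys the enemy on death.
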(event `self.ReceiveBeginPlay`
  (bind _aswbp_health_bar (cast `/Game/ThirdPerson/Blueprints/WBP_HealthBar` (`WidgetComponent.GetWidget` (`self.HealthBar`))))
  (bind _output_get (set `self.As WBP Health Bar` _aswbp_health_bar))
  (`/Game/ThirdPerson/Blueprints/WBP_HealthBar.SetHP` _output_get (`self.Health`))
  (add `AIPerceptionComponent.OnTargetPerceptionForgotten` (`self.AIPerception`) (delegate `OnTargetPerceptionForgotten_Event`))
  (bind _outactors (`GameplayStatics.GetAllActorsWithTag` (`self.Tag`) :!label _label))
  (`|AIMoveTo` self (0.0 0.0 0.0) (`KismetArrayLibrary.Array_Random` _outactors) 70.0
    (:`OnSuccess`
      (`KismetSystemLibrary.Delay` 1.0)
      (goto _label))))

(event `OnTargetPerceptionForgotten_Event`
  (params (Actor :type "Actor Object Reference")))

(event `self.AIPerception.OnTargetPerceptionForgotten`
  (params (Actor :type "Actor Object Reference"))
  (cast `/Game/ThirdPerson/Blueprints/BP_ThirdPersonCharacter` Actor)
  (set `CharacterMovementComponent.MaxWalkSpeed` 300.0 (`self.CharacterMovement`))
  (goto _label))

(event `self.Health.OnHealthUpdate`
  (bind _as_wbp_health_bar (`self.As WBP Health Bar`))
  (`/Engine/EditorBlueprintResources/StandardMacros.IsValid` _as_wbp_health_bar
    (:`Is Valid`
      (`/Game/ThirdPerson/Blueprints/WBP_HealthBar.SetHP` _as_wbp_health_bar (`self.Health`)))))

(event `self.Health.OnDeath`
  (`self.K2_DestroyActor`))

(event `self.AIPerception.OnTargetPerceptionUpdated`
  (params (Actor :type "Actor Object Reference") (Stimulus :type "AIStimulus Structure"))
  (bind _returnvalue (`self.K2_GetActorLocation`))
  (bind _asbp_third_person_character (cast `/Game/ThirdPerson/Blueprints/BP_ThirdPersonCharacter` Actor))
  (set `CharacterMovementComponent.MaxWalkSpeed` 650.0 (`self.CharacterMovement`))
  (`|AIMoveTo` self (0.0 0.0 0.0) _asbp_third_person_character 70.0
    (:`OnSuccess`
      (if (`self.CanAttack?`)
        (`|PlayMontage` (`self.Mesh`) "/Game/Enemy/AM_ChargedAttack_Enemy.AM_ChargedAttack_Enemy"
          (:`then`
            (set `self.CanAttack?` false))
          (:`OnCompleted`
            (set `self.CanAttack?` true :!label _label_2))
          (:`OnInterrupted`
            (goto _label_2))
          (:`OnNotifyBegin`
            (bind (_outhit _returnvalue_2) (`KismetSystemLibrary.SphereTraceSingleForObjects` :`Start` _returnvalue :`End` (+ _returnvalue (* (`KismetMathLibrary.GetForwardVector` (`self.K2_GetActorRotation`)) 200.0)) :`Radius` 20.0 :`ObjectTypes` (`|MakeArray` "ObjectTypeQuery3" :!type "EObjectTypeQuery Enum") :`DrawDebugType` "ForDuration" :`DrawTime` 0.5))
            (if _returnvalue_2
              (bind _asbp_third_person_character_2 (cast `/Game/ThirdPerson/Blueprints/BP_ThirdPersonCharacter` (`.HitActor` (`GameplayStatics.BreakHitResult` _outhit))))
              (`HealthComponent.TakeDamage` (`CDPR_00Character.HealthComp` _asbp_third_person_character_2) 30))))))))

(fn `UserConstructionScript`)